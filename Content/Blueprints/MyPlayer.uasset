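; MyPlayer is the player Blueprint for a physics-driven Ball that constantly moves along X at MoveSpeed.
; Enhanced Input Move sets TurnValue from TurnSpeed, and Tick writes it as Y velocity while preserving Z.
; Jump sets Z to JumpSpeed and Y to raw TurnSpeed, which the next Tick replaces with TurnValue.
; No ground check gates the jump, and the overlap events are empty.
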(event OnComponentBeginOverlap(Ball)
  (params (OverlappedComponent :type Primitive%20Component%20Object%20Reference) (OtherActor :type Actor%20Object%20Reference) (OtherComp :type Primitive%20Component%20Object%20Reference) (OtherBodyIndex :type Integer) (bFromSweep :type Boolean) (SweepResult :type Hit%20Result%20Structure%20%28by%20ref%29)))

(event Input|EnhancedActionEvents|EnhancedInputActionMove
  (params (ActionValue :type Float%20%28double-precision%29) (ElapsedSeconds :type Float%20%28double-precision%29) (TriggeredSeconds :type Float%20%28double-precision%29) (InputAction :type Input%20Action%20Object%20Reference :default "/Game/Inputs/Move.Move"))
  (:Triggered
    (Variables|Default|SetTurnValue (* ActionValue (Variables|Default|GetTurnSpeed))))
  (:Completed
    (Variables|Default|SetTurnValue 0.0)))

(event Input|EnhancedActionEvents|EnhancedInputActionJump
  (params (ActionValue :type Boolean) (ElapsedSeconds :type Float%20%28double-precision%29) (TriggeredSeconds :type Float%20%28double-precision%29) (InputAction :type Input%20Action%20Object%20Reference :default "/Game/Inputs/Jump.Jump"))
  (:Triggered
    (Physics|SetPhysicsLinearVelocity (Variables|Default|GetBall) (Math|Vector|MakeVector (Variables|Default|GetMoveSpeed) (Variables|Default|GetTurnSpeed) (Variables|Default|GetJumpSpeed)) false "None")))

(event EventBeginPlay
  (Physics|SetPhysicsLinearVelocity (Variables|Default|GetBall) (Math|Vector|MakeVector (Variables|Default|GetMoveSpeed) 0.0 0.0) false "None"))

(event Collision|EventActorBeginOverlap
  (params (OtherActor :type Actor%20Object%20Reference)))

(event EventTick
  (params (DeltaSeconds :type Float%20%28single-precision%29))
  (bind _ball (Variables|Default|GetBall))
  (bind _returnvalue (Physics|GetPhysicsLinearVelocity _ball "None"))
  (Physics|SetPhysicsLinearVelocity _ball (Math|Vector|MakeVector (Variables|Default|GetMoveSpeed) (Variables|Default|GetTurnValue) (.z _returnvalue)) false "None"))

(fn ConstructionScript)